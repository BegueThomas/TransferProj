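; BP_FoliageLight is an actor whose point light reacts to how close the player is.
; Each Tick, while it overlaps the player pawn, a clamped range map converts their distance into light intensity, brightest up close.
; The fade range derives from the Sphere component's radius plus a margin.
; Intensity is not updated outside the overlap, so the light keeps its last value.
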(event `self.ReceiveActorBeginOverlap`
  (params (OtherActor :type "Actor Object Reference")))

(event `self.ReceiveTick`
  (params (DeltaSeconds :type "Float (single-precision)"))
  (bind _returnvalue (`GameplayStatics.GetPlayerPawn` 0))
  (if (`self.IsOverlappingActor` _returnvalue)
    (`LightComponent.SetIntensity` (`self.PointLight`) (`KismetMathLibrary.MapRangeClamped` (`self.GetDistanceTo` _returnvalue) 0.0 (+ (`SphereComponent.SphereRadius` (`self.Sphere`)) 100.0) 10000.0))))

(fn `UserConstructionScript`)